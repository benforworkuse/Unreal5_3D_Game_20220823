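; BP_Door is a door that opens when the player overlaps its trigger box while carrying enough boxes.
; On overlap it casts to BP_Player and compares the collected box count with the player's maximum.
; If enough, the 開門 timeline drives the wall mesh's relative Z to open it; otherwise it prints a "not enough boxes" message.
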(event OnComponentBeginOverlap(Box-Col)
  (params (OverlappedComponent :type Primitive%20Component%20Object%20Reference) (OtherActor :type Actor%20Object%20Reference) (OtherComp :type Primitive%20Component%20Object%20Reference) (OtherBodyIndex :type Integer) (bFromSweep :type Boolean) (SweepResult :type Hit%20Result%20Structure%20%28by%20ref%29))
  (bind _asbp_player (Utilities|Casting|CastToBP_Player OtherActor)) ; 轉換為玩家藍圖，如果是就從第一個出口
  (if (>= (Variables|/Game/BP/BP_Player.BP_Player_C|Get取得箱子數量 _asbp_player) (Variables|/Game/BP/BP_Player.BP_Player_C|Get最大箱子數量 _asbp_player))
    (bind _上下開門z軸 (Timeline|開門 Play)
      (:Update
        (Transformation|SetRelativeLocation (Variables|Default|GetSM_wall_10) (Math|Vector|MakeVector 0.0 0.0 _上下開門z軸) false false)))
    (else
      (Development|PrintString "箱子不夠"))))

(fn ConstructionScript)